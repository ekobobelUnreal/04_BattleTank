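; Player-controllable tank Blueprint that binds input for driving, camera aiming and firing.
; On BeginPlay it passes the Barrel and Turret components to the tank's reference setters.
; Aim axes rotate the azimuth gimbal and spring arm, scaled by frame time, while left mouse or gamepad face-left fires.
; Forward input feeds the movement component, and track throttle axes drive opposite-named tracks (Left to TankTrackRight, Right to TankTrackLeft).
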(event `self.ReceiveBeginPlay`
  (`self.SetBarrelReference` (`self.Barrel`))
  (`self.SetTurretReference` (`self.Turret`)))

(event `InputAxis|AimAzimuth`
  (params (AxisValue :type "Float (single-precision)"))
  ;[1 1 1] Aiming Input Binding
  (`SceneComponent.K2_AddLocalRotation` (`self.Azimuth Gimbal`) (`KismetMathLibrary.MakeRotator` 0.0 0.0 (* AxisValue (`GameplayStatics.GetWorldDeltaSeconds`) 100.0)) false false))

(event `InputAxis|AimElevation`
  (params (AxisValue :type "Float (single-precision)"))
  ;[1 1 1] Aiming Input Binding
  (`SceneComponent.K2_AddLocalRotation` (`self.SpringArm`) (`KismetMathLibrary.MakeRotator` 0.0 (* AxisValue (`GameplayStatics.GetWorldDeltaSeconds`) 100.0)) false false))

(event `InputAxis|Left Track Throttle`
  (params (AxisValue :type "Float (single-precision)"))
  ;[1 1 1] Movement Input Binding
  (`TankTrack.SetThrottle` (`self.TankTrackRight`) AxisValue))

(event `InputAxis|Right Track Throttle`
  (params (AxisValue :type "Float (single-precision)"))
  ;[1 1 1] Movement Input Binding
  (`TankTrack.SetThrottle` (`self.TankTrackLeft`) AxisValue))

(event `Key|Gamepad_FaceButton_Left`
  (params (Key :type "Key Structure" :default "AnyKey"))
  ;[1 1 1] Aiming Input Binding
  (:`Pressed`
    (`self.Fire`)))

(event `InputAxis|Move Forward`
  (params (AxisValue :type "Float (single-precision)"))
  ;[1 1 1] Movement Input Binding
  (`TankMovementComponent.IntendMoveForward` (`self.TankMovementComponent`) AxisValue))

(event `Key|LeftMouseButton`
  (params (Key :type "Key Structure" :default "AnyKey"))
  ;[1 1 1] Aiming Input Binding
  (:`Pressed`
    (`self.Fire`)))

(fn `UserConstructionScript`)